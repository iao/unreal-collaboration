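; BPPlayerController is a player controller Blueprint that holds user info, including a username and rank, and displays it as debug text.
; UponInfoChanged prints the Info, Rank and Username to screen, coloring the rank red when the user has selector authority and black otherwise.
; HasSelectorAuthority grants that authority by comparing the Rank string to "admin".
; BeginPlay, Tick and the construction script are empty.
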(event EventBeginPlay)

(event EventTick
  (params (DeltaSeconds :type Float%20%28single-precision%29)))

(event EventUponInfoChanged
  (bind _duration (Variables|Default|GetDuration))
  (Development|PrintString (Utilities|String|ToString(Integer) (Variables|Default|Getinfo)) true true "(R=0.000000,G=0.000000,B=0.000000,A=1.000000)" _duration)
  (bind _returnvalue (CallFunction|HasSelectorAuthority))
  (Development|PrintString (Variables|Default|Getrank) true true (Math|Color|SelectColor :A "(R=1.000000,G=0.000000,B=0.000000,A=1.000000)" :bPickA _returnvalue) _duration)
  (Development|PrintString (Variables|Default|Getusername) true true "(R=0.000000,G=0.660000,B=1.000000,A=1.000000)" _duration))

(fn ConstructionScript)

(fn HasSelectorAuthority
  (return (Utilities|Enum|Equal(Enum) (Variables|Default|Getrank) "admin")))