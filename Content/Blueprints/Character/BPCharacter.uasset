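; BPCharacter is a character Blueprint that shows user info on screen when that info changes.
; UponInfoChanged prints Info in green, Username in red for admins or white otherwise, and Rank in the default color.
; It also applies the same admin-based color to the TextRender of TextActor, without setting its text.
; BeginPlay, overlap, Tick and the construction script hold no logic.
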(event EventBeginPlay)

(event Collision|EventActorBeginOverlap
  (params (OtherActor :type Actor%20Object%20Reference)))

(event EventTick
  (params (DeltaSeconds :type Float%20%28single-precision%29)))

(event EventUponInfoChanged
  (bind _isadmin (Variables|Default|GetisAdmin))
  (bind _duration (Variables|Default|GetDuration))
  (bind _returnvalue (Math|Color|SelectColor "(R=1.000000,G=0.000000,B=0.000000,A=1.000000)" "(R=1.000000,G=1.000000,B=1.000000,A=1.000000)" _isadmin))
  (Development|PrintString (Utilities|String|ToString(Integer) (Variables|Default|Getinfo)) true true "(R=0.000000,G=1.000000,B=0.000000,A=1.000000)" _duration)
  (Development|PrintString (Variables|Default|Getusername) true true _returnvalue _duration)
  (Development|PrintString (Variables|Default|Getrank) true true "(R=0.000000,G=0.660000,B=1.000000,A=1.000000)" _duration)
  (Rendering|Components|TextRender|SetTextRenderColor (Variables|/Script/Engine.TextRenderActor|GetTextRender (Variables|Default|GetTextActor)) (Math|Conversions|ToColor(LinearColor) _returnvalue)))

(fn ConstructionScript)